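; BP_ghost is an enemy ghost actor that flies from its starting position to the first player's pawn.
; It stores both on BeginPlay, then each Tick refreshes the player's position and plays a Timeline.
; Timeline curves drive the lerp toward that moving target, a Height-scaled vertical offset and a wobble on Y and Z.
; Its rotation follows the look-at direction from the start position, not its current one.
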(event EventBeginPlay
  (Variables|Default|SetStart_position (Transformation|GetActorLocation))
  (Variables|Default|SetPlayer (Game|Player|GetPlayerPawn 0)))

(event Collision|EventActorBeginOverlap
  (params (OtherActor :type Actor%20Object%20Reference)))

(event EventTick
  (params (DeltaSeconds :type Float%20%28single-precision%29))
  (Variables|Default|Setplayer_posit (Transformation|GetActorLocation (Variables|Default|GetPlayer)))
  (bind (_direction _alpha _alpha_height_ _oscilacion) (Timeline|Timeline Play)
    (:Update
      (Transformation|SetActorLocation (Math|Vector|MakeVector (.x (Math|Vector|Lerp(Vector) (Variables|Default|GetStart_position) (Variables|Default|Getplayer_posit) _alpha)) (+ (.y (Math|Vector|Lerp(Vector) (Variables|Default|GetStart_position) (Variables|Default|Getplayer_posit) _alpha)) (* _oscilacion 15.0)) (+ (.z (Math|Vector|Lerp(Vector) (Variables|Default|GetStart_position) (Variables|Default|Getplayer_posit) _alpha)) (* _alpha_height_ (Variables|Default|GetHeight)) (* _oscilacion 2e+01))) false false)
      (Transformation|SetActorRotation (Math|Rotator|FindLookatRotation (Variables|Default|GetStart_position) (Variables|Default|Getplayer_posit))))))

(fn ConstructionScript)