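; BP_zombi is a zombie enemy Blueprint that gives the character a stuttering, stop-and-go walk.
; From BeginPlay, an endless chain of fixed Delay nodes alternates CharacterMovement MaxWalkSpeed between the Walkspeedo variable and zero in an uneven repeating rhythm.
; The graph only modulates speed and contains no targeting, attack or movement input logic.
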(event EventBeginPlay
  (bind _charactermovement (Variables|Character|GetCharacterMovement))
  (bind _charactermovement_2 (Variables|Character|GetCharacterMovement))
  (Variables|/Script/Engine.CharacterMovementComponent|SetMaxWalkSpeed _charactermovement_2 (Variables|Default|Getwalkspeedo))
  (Utilities|FlowControl|Delay 0.45 :!label _label)
  (Variables|/Script/Engine.CharacterMovementComponent|SetMaxWalkSpeed _charactermovement_2 0.0)
  (Utilities|FlowControl|Delay 0.55)
  (Variables|/Script/Engine.CharacterMovementComponent|SetMaxWalkSpeed _charactermovement (Variables|Default|Getwalkspeedo))
  (Utilities|FlowControl|Delay 1.4)
  (Variables|/Script/Engine.CharacterMovementComponent|SetMaxWalkSpeed _charactermovement 0.0)
  (Utilities|FlowControl|Delay 0.6)
  (Variables|/Script/Engine.CharacterMovementComponent|SetMaxWalkSpeed _charactermovement (Variables|Default|Getwalkspeedo))
  (Utilities|FlowControl|Delay 1.07)
  (goto _label))

(event Collision|EventActorBeginOverlap
  (params (OtherActor :type Actor%20Object%20Reference)))

(event EventTick
  (params (DeltaSeconds :type Float%20%28single-precision%29)))

(fn ConstructionScript)