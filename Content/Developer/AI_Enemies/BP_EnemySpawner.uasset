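; Enemy spawner actor that periodically spawns one of two enemy classes at its own transform.
; BeginPlay starts a looping timer on SpawnEnemy, with an interval randomized once between the min and max settings.
; Flags select a random class or a fixed one (Ghost or the other), and optional group spawning.
; A counter loops groups back to the spawn node: random groups spawn immediately, single-type groups with a short delay between spawns.
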(event Custom|Spawn%20Enemy
  (bind _returnvalue (Transformation|GetActorTransform))
  (bind _enemyclasses (Variables|Default|GetEnemyClasses))
  (if (Variables|Default|GetAleatorio?)
    ;[0.15 0.15 0.15 0.5] Funcionalidad para Spawnear cualquier tipo de enemigo
    (Game|SpawnActorfromClass (Utilities|Array|Get(acopy) (Variables|Default|GetEnemyClasses) (Math|Random|RandomIntegerinRange 0 1)) (Transformation|GetActorTransform) "AdjustIfPossibleButAlwaysSpawn" "MultiplyWithRoot" 0 0 :!label _label)
    ;;[0.15 0.15 0.15 0.5] Bucle para spawnear por grupos
    (if (Variables|Default|GetGrupo?)
      (if (< (Variables|Default|GetEnemigosActuales) (- (Variables|Default|GetGrupo%20Numero) 1))
        (Variables|Default|SetEnemigosActuales (+ (Variables|Default|GetEnemigosActuales) 1))
        (goto _label)
        (else
          (Variables|Default|SetEnemigosActuales 0))))
    (else
      ;[0.15 0.15 0.15 0.5] Funcionalidad para Spawnear solo un tipo de enemigo
      (if (Variables|Default|GetGhost?)
        (Game|SpawnActorfromClass (Utilities|Array|Get(acopy) _enemyclasses) _returnvalue "AdjustIfPossibleButAlwaysSpawn" "MultiplyWithRoot" 0 0 :!label _label_2)
        ;;[0.15 0.15 0.15 0.5] Bucle para spawnear por grupos de un mismo enemigo
        (if (Variables|Default|GetGrupo?) :!label _label_3
          (if (< (Variables|Default|GetEnemigosActuales) (- (Variables|Default|GetGrupo%20Numero) 1))
            (Variables|Default|SetEnemigosActuales (+ (Variables|Default|GetEnemigosActuales) 1))
            (Utilities|FlowControl|Delay 0.5)
            (if (Variables|Default|GetGhost?)
              (goto _label_2)
              (else
                (Game|SpawnActorfromClass (Utilities|Array|Get(acopy) _enemyclasses 1) _returnvalue "AdjustIfPossibleButAlwaysSpawn" "MultiplyWithRoot" 0 0 :!label _label_4)
                (goto _label_3)))
            (else
              (Variables|Default|SetEnemigosActuales 0))))
        (else
          (goto _label_4))))))

(event EventBeginPlay
  ;[0.15 0.15 0.15 0.5] Evento Principal e Intervalos de Spawn
  (Utilities|Time|SetTimerbyEvent (delegate Custom|Spawn%20Enemy) (Math|Random|RandomFloatinRange (Variables|Default|GetMin-SpawnInterval) (Variables|Default|GetMax-SpawnInterval)) true))

(fn ConstructionScript)