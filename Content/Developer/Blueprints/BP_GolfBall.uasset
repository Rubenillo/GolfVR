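; BP_GolfBall is a golf ball actor that shows a marker icon when the player camera is far from it.
; A looping timer started on BeginPlay refreshes the icon widget at a configurable interval instead of on Tick.
; Each refresh turns the widget toward the camera, scales it up with camera distance within clamped limits, and shows it only beyond the render distance threshold.
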(event Custom|UpdateIcon
  (bind _returnvalue (Game|GetPlayerCameraManager 0))
  (bind _iconballwidget (Variables|Default|GetIconBallWidget))
  (bind _iconballwidget_2 (Variables|Default|GetIconBallWidget))
  ;[0.15 0.3565 0.05234 0.5] RotationUpdate
  (Transformation|SetWorldRotation _iconballwidget (Math|Rotator|FindLookatRotation (Transformation|GetWorldLocation _iconballwidget) (Camera|GetCameraLocation _returnvalue)) false false)
  ;[0.15 0.15 0.15 0.5] Update Scale Based on Distance
  (bind _output_get (Variables|Default|SetDistanceToPlayer (Transformation|GetDistanceTo _returnvalue)))
  (Transformation|SetWorldScale3D (Variables|Default|GetIconBallWidget) (Math|Vector|MakeVector (Math|Float|MapRangeClamped _output_get 0.0 2e+03 0.01 0.5) (Math|Float|MapRangeClamped _output_get 0.0 2e+03 0.01 0.5) (Math|Float|MapRangeClamped _output_get 0.0 2e+03 0.01 0.5)))
  ;[0.15 0.15 0.15 0.5] UpdateDistanceVisibility
  (if (> (Variables|Default|GetDistanceToPlayer) (Variables|Default|GetIconRenderDistance))
    (Rendering|SetVisibility _iconballwidget_2 true false)
    (else
      (Rendering|SetVisibility _iconballwidget_2 false false))))

(event EventBeginPlay
  (Utilities|Time|SetTimerbyEvent (delegate Custom|UpdateIcon) (Variables|Default|GetRefreshIconTimer) true))

(fn ConstructionScript)